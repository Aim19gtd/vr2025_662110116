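; House_BP is a house Blueprint that lets the player switch on its lights when standing nearby.
; A Box trigger shows a text render prompt and enables input on overlap, then hides the prompt and disables input when the overlap ends.
; While input is enabled, pressing F prints a debug message and makes six spotlights visible, with no logic to switch them off again.
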(event OnComponentBeginOverlap(Box)
  (params (OverlappedComponent :type Primitive%20Component%20Object%20Reference) (OtherActor :type Actor%20Object%20Reference) (OtherComp :type Primitive%20Component%20Object%20Reference) (OtherBodyIndex :type Integer) (bFromSweep :type Boolean) (SweepResult :type Hit%20Result%20Structure%20%28by%20ref%29))
  ;[1 0 0] Comment
  (Rendering|SetVisibility (Variables|Default|GetTextRender1) true false)
  (Input|EnableInput (Game|GetPlayerController 0)))

(event OnComponentEndOverlap(Box)
  (params (OverlappedComponent :type Primitive%20Component%20Object%20Reference) (OtherActor :type Actor%20Object%20Reference) (OtherComp :type Primitive%20Component%20Object%20Reference) (OtherBodyIndex :type Integer))
  ;[1 0 0] Comment
  (Rendering|SetVisibility (Variables|Default|GetTextRender1) false false)
  (Input|DisableInput (Game|GetPlayerController 0)))

(event Input|KeyboardEvents|F
  (params (Key :type Key%20Structure :default "None"))
  ;[0 0 0] Comment
  (:Pressed
    (Development|PrintString "Turn On")
    (Rendering|SetVisibility (Variables|Default|GetSpotLight1) true false)))

(fn ConstructionScript)